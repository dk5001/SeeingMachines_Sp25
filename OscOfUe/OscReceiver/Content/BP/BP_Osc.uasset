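; BP_Osc is an OSC receiver that switches its point light between bright and dim from network messages.
; On BeginPlay it starts a listening OSC server on a hard-coded IP and port, binds a message event and sets the light dim.
; OscIn matches the last segment of the message address against Brightness, then uses the first integer to pick the intensity, printing ON or OFF.
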(event Custom|OscIn
  (params (Message :type OSC%20Message%20Structure%20%28by%20ref%29) (IPAddress :type String) (Port :type Integer))
  (bind _pointlight (Variables|Default|GetPointLight))
  (bind _output_get (Variables|Default|SetOscMessages Message))
  (bind _returnvalue (Class|OSCManager|GetOSCMessageAddress _output_get))
  (bind _returnvalue_2 (Class|OSCManager|GetOSCAddressFullPath _returnvalue))
  (switch string (.RightS (Utilities|String|Split _returnvalue_2 "/" "IgnoreCase" "FromEnd"))
    (:brightness
      (bind _value (Class|OSCManager|GetInt32 (Variables|Default|GetOscMessages)))
      (bind _output_get_2 (Variables|Default|SetValue _value))
      (if (== _output_get_2 1)
        (Development|PrintString "ON")
        (Rendering|Components|Light|SetIntensity _pointlight 5e+03)
        (else
          (Development|PrintString "OFF")
          (Rendering|Components|Light|SetIntensity _pointlight 5e+01))))))

(event EventBeginPlay
  (bind _returnvalue (Class|OSCManager|CreateOSCServer "192.168.1.164" 3030 false true "" 0))
  (bind _output_get (Variables|Default|SetOscServer _returnvalue))
  (EventDispatchers|BindEventtoOnOscMessageReceived _output_get (EventDispatchers|CreateEvent :!event Custom|OscIn))
  (Rendering|Components|Light|SetIntensity (Variables|Default|GetPointLight) 5e+01))

(fn ConstructionScript)